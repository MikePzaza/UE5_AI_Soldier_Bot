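; BoxActor is an interactive physics box that responds to key input while something overlaps it.
; Beginning an overlap enables input for player controller 0 and shows its Widget component; ending it disables input and hides the widget, with no check on the overlapping actor.
; While input is enabled, E launches the StaticMesh upward with an impulse and R spins it around the vertical axis with an angular impulse.
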(event EventBeginPlay)

(event Collision|EventActorBeginOverlap
  (params (OtherActor :type Actor%20Object%20Reference))
  (bind _returnvalue (Game|GetPlayerController 0))
  (Input|EnableInput _returnvalue)
  (Rendering|SetVisibility (Variables|Default|GetWidget) true false))

(event EventTick
  (params (DeltaSeconds :type Float%20%28single-precision%29)))

(event Collision|EventActorEndOverlap
  (params (OtherActor :type Actor%20Object%20Reference))
  (bind _returnvalue (Game|GetPlayerController 0))
  (Input|DisableInput _returnvalue)
  (Rendering|SetVisibility (Variables|Default|GetWidget) false false))

(event Input|KeyboardEvents|E
  (params (Key :type Key%20Structure :default "None"))
  (:Pressed
    (Physics|AddImpulse (Variables|Default|GetStaticMesh) "0.000000,0.000000,5000.000000" "None" false)))

(event Input|KeyboardEvents|R
  (params (Key :type Key%20Structure :default "None"))
  (:Pressed
    (Class|PrimitiveComponent|AddAngularImpulseinDegrees (Variables|Default|GetStaticMesh) "0.000000,0.000000,2378000.000000" "None" false)))

(fn ConstructionScript)